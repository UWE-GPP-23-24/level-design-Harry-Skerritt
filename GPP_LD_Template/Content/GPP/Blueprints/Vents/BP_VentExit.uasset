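; Vent exit trigger Blueprint that advances the mission and starts moving lava when the player reaches it.
; Player overlap with its box stops the fan on every entry.
; The first pass completes the current mission, waits briefly, starts the next one, then starts the lava.
; A flag skips the mission step on later overlaps, but it is only set after the delay.
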(event `self.ReceiveBeginPlay`
  (set `self.MissionTriggered` false))

(event `self.Box.OnComponentBeginOverlap`
  (params (OverlappedComponent :type "PrimitiveComponent Object Reference") (OtherActor :type "Actor Object Reference") (OtherComp :type "PrimitiveComponent Object Reference") (OtherBodyIndex :type Integer) (bFromSweep :type Boolean) (SweepResult :type "HitResult Structure (by ref)"))
  (bind _missionmanager (`self.MissionManager`))
  (cast `/Game/GPP/Blueprints/Essential/BP_PlayerCharacter` OtherActor)
  (`/Game/GPP/Blueprints/Vents/BP_Fan.StopSpinning` (`self.Fan`))
  (if (not (`self.MissionTriggered`))
    (`/Game/GPP/Blueprints/Missions/BP_MissionManager.CompleteMission` _missionmanager)
    (`KismetSystemLibrary.Delay` 1.0)
    (`/Game/GPP/Blueprints/Missions/BP_MissionManager.StartNextMission` _missionmanager)
    (set `self.MissionTriggered` true))
  (`/Game/GPP/Blueprints/ServerRoom/BP_MovingLava.StartMoving` (`self.MovingLava`)))

(fn `UserConstructionScript`)