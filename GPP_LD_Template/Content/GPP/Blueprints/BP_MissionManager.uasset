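; BP_MissionManager runs a linear sequence of missions, showing one at a time on screen through a WBP_Mission widget.
; GetMission finds the MissionsData row whose position matches an index, and its text and completion flag feed the new widget.
; StartNextMission increments the index and replaces the widget.
; CompleteMission updates the widget and sets completion on a temporary struct, without writing it back to the DataTable.
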(fn `CompleteMission`
  ; Update Mission Visually
  (`/Game/GPP/Widgets/Mission/WBP_Mission.CompleteMission` (`self.MissionWidget`))
  ; Update Mission Data
  (bind _mission (`self.GetMission` (`self.CurrentMissionIndex`)))
  (setmembers `/Game/GPP/Blueprints/S_MissionData` :`StructRef` (make `/Game/GPP/Blueprints/S_MissionData` true (`.MissionText_4_5343017E429DB46ABC0DD0AB51AB7B5E` (break `/Game/GPP/Blueprints/S_MissionData` _mission)))))

(fn `GetMission`
  (params (Index :type Integer))
  (returns (Mission :type "/Game/GPP/Blueprints/S_MissionData Structure"))
  (bind _missionsdata (`self.MissionsData`))
  (bind _outrownames (`DataTableFunctionLibrary.GetDataTableRowNames` _missionsdata))
  (bind (_arrayindex _arrayelement) (`/Engine/EditorBlueprintResources/StandardMacros.ReverseForEachLoop` _outrownames)
    (:`LoopBody`
      (if (== _arrayindex Index)
        (bind _returnvalue (`|GetDataTableRow` _missionsdata _arrayelement)
          (:`then`
            _)
          (:`RowNotFound`
            _))
        (return _returnvalue)))))

(fn `StartInitialMission`
  (bind _mission (`self.GetMission` (`self.CurrentMissionIndex`)))
  (bind (_missioncompleted _missiontext) (break `/Game/GPP/Blueprints/S_MissionData` _mission))
  (bind _returnvalue (`|CreateWidget` "/Game/GPP/Widgets/Mission/WBP_Mission.WBP_Mission_C" (`GameplayStatics.GetPlayerController` 0) _missiontext _missioncompleted))
  (bind _output_get (set `self.MissionWidget` _returnvalue))
  (`UserWidget.AddToViewport` _output_get 0))

(fn `StartNextMission`
  (`/Engine/EditorBlueprintResources/StandardMacros.IncrementInt` (`self.CurrentMissionIndex`)
    (:`  `
      (`Widget.RemoveFromParent` (`self.MissionWidget`))
      (`self.StartInitialMission`))))

(fn `UserConstructionScript`)