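; BP_ElevatorDoors is a two-panel sliding elevator door that opens and closes on request through OpenDoor and CloseDoor events.
; An IsOpen flag ignores repeated calls, and the OpenCloseDoor timeline plays forward to open and reverses to close.
; Its DoorTrack curve lerps the left and right door meshes apart along their relative X axis in mirrored motion.
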(event `Open Door`
  (if (not (`self.IsOpen`))
    (set `self.IsOpen` true)
    (bind (_direction _door_track) (`Timeline|Open / Close Door` :!label _label)
      (:`Update`
        (`SceneComponent.K2_SetRelativeLocation` (`self.DoorL`) (`KismetMathLibrary.MakeVector` (`KismetMathLibrary.Lerp` -25.0 -75.0 _door_track)) false false)
        (`SceneComponent.K2_SetRelativeLocation` (`self.DoorR`) (`KismetMathLibrary.MakeVector` (`KismetMathLibrary.Lerp` 25.0 75.0 _door_track)) false false)))))

(event `Close Door`
  (if (`self.IsOpen`)
    (set `self.IsOpen` false)
    (goto _label :!via `Reverse`)))

(fn `UserConstructionScript`)