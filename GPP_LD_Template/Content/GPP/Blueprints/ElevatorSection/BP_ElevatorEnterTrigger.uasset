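; Trigger volume for the elevator section that runs a fake elevator ride when the player character enters it.
; On overlap it turns off a light, completes the current mission, closes the elevator doors and spawns servers through the ServerManager.
; A delayed loop then steps the floor sign from start to end floor to imply movement, before opening the exit doors.
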(event `self.Box.OnComponentBeginOverlap`
  (params (OverlappedComponent :type "PrimitiveComponent Object Reference") (OtherActor :type "Actor Object Reference") (OtherComp :type "PrimitiveComponent Object Reference") (OtherBodyIndex :type Integer) (bFromSweep :type Boolean) (SweepResult :type "HitResult Structure (by ref)"))
  (cast `/Game/GPP/Blueprints/Essential/BP_PlayerCharacter` OtherActor)
  (`LightComponent.SetIntensity` (`Light.LightComponent` (`self.Light`)) 0.0)
  ; Mission
  (`/Game/GPP/Blueprints/Missions/BP_MissionManager.CompleteMission` (`self.MissionManager`))
  ; Door Closing
  (`KismetSystemLibrary.Delay` 1.0)
  (`/Game/GPP/Blueprints/ElevatorSection/BP_ElevatorDoors.Close Door` (`self.ElevatorDoors`))
  (`KismetSystemLibrary.Delay` (* (`self.SignDelay`) 0.5))
  (`/Game/GPP/Blueprints/ServerRoom/ServerRack/BP_ServerRackManager.SpawnServers` (`self.ServerManager`))
  ; Lift 'Movement'
  (bind _output_get (set `self.CurrentFloor` (`self.StartingFloor`)))
  (if (<= _output_get (- (`self.EndFloor`) 1)) :!label _label
    ;; Loop Body
    (bind _result (`/Engine/EditorBlueprintResources/StandardMacros.IncrementInt` (`self.CurrentFloor`))
      (:`  `
        (bind _output_get_2 (set `self.CurrentFloor` _result))
        (`KismetSystemLibrary.Delay` (`self.SignDelay`))
        (`/Game/GPP/Blueprints/ElevatorSection/BP_ElevatorSign.SetFloorNo` (`self.ElevatorSign`) (`KismetTextLibrary.Conv_IntToText` _output_get_2))
        (goto _label)))
    (else
      ;; Loop Complete
      (`KismetSystemLibrary.Delay` 0.2)
      (`/Game/GPP/Blueprints/ElevatorSection/BP_ElevatorDoors.Open Door` (`self.ElevatorDoorsOut`)))))

(fn `UserConstructionScript`)