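; BP_Vent is a server room vent that swings open on its hinge when triggered.
; OpenVent sets a swinging flag, and Tick then eases the Hinge's relative rotation toward TargetRot with RInterpTo until it arrives and the flag clears.
; ResetVent stops the swing and snaps the hinge to zero relative rotation.
; BeginPlay stores the hinge's world rotation in StartRot, which these graphs never read.
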(event `ResetVent`
  ; Reset
  (set `self.IsSwinging` false)
  (`SceneComponent.K2_SetRelativeRotation` :`self` (`self.Hinge`)))

(event `self.ReceiveBeginPlay`
  ; Init
  (set `self.StartRot` (`SceneComponent.K2_GetComponentRotation` (`self.Hinge`))))

(event `OpenVent`
  ; Trigger
  (set `self.IsSwinging` true))

(event `self.ReceiveTick`
  (params (DeltaSeconds :type "Float (single-precision)"))
  (bind _targetrot (`self.TargetRot`))
  (bind _returnvalue (`KismetMathLibrary.RInterpTo` (`SceneComponent.RelativeRotation` (`self.Hinge`)) _targetrot DeltaSeconds 5.0))
  ; Handle Opening
  (if (`self.IsSwinging`)
    (`SceneComponent.K2_SetRelativeRotation` (`self.Hinge`) _returnvalue false false)
    (if (== _returnvalue _targetrot)
      (set `self.IsSwinging` false))))

(fn `UserConstructionScript`)