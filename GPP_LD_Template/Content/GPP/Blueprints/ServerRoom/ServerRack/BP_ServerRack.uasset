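; Server rack actor that fills itself with a randomized stack of server actors.
; SpawnServers rolls randomly for each slot, leaving it empty or spawning BP_Server or the rarer BP_Server2, offset along the rack's up vector by slot height.
; Spawned servers are tracked in one array per type.
; DestoryServers destroys them, removing array entries during forward iteration, which can skip elements.
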(event `SpawnServers`
  (bind (_returnvalue_location _returnvalue_rotation _returnvalue_scale) (`KismetMathLibrary.BreakTransform` (`self.GetTransform`)))
  ; SpawnServers
  (for _index (range (+ (`self.MaxSlots`) 1))
    (switch `int` (`KismetMathLibrary.RandomIntegerInRange` 0 10)
      (:`0`
        (bind _returnvalue (+ _returnvalue_location (* (`self.GetActorUpVector`) (* _index (`self.SlotHeight`)))))
        (bind _returnvalue_2 (`|SpawnActorFromClass` "/Game/GPP/Blueprints/ServerRoom/ServerRack/BP_Server.BP_Server_C" (`KismetMathLibrary.MakeTransform` _returnvalue _returnvalue_rotation _returnvalue_scale) "AlwaysSpawn" "MultiplyWithRoot" null null :!label _label))
        (`KismetArrayLibrary.Array_Add` (`self.Servers_1`) _returnvalue_2))
      (:`1`
        (goto _label))
      (:`2`
        (goto _label))
      (:`5`
        (bind _returnvalue_3 (`|SpawnActorFromClass` "/Game/GPP/Blueprints/ServerRoom/ServerRack/BP_Server2.BP_Server2_C" (`KismetMathLibrary.MakeTransform` _returnvalue _returnvalue_rotation _returnvalue_scale) "AlwaysSpawn" "MultiplyWithRoot" null null :!label _label_2))
        (`KismetArrayLibrary.Array_Add` (`self.Servers_2`) _returnvalue_3))
      (:`6`
        (goto _label_2)))))

(event `DestoryServers`
  (bind _servers_1 (`self.Servers_1`))
  (bind _servers_2 (`self.Servers_2`))
  ; Destory Servers
  (`|ExecutionSequence`
    (:`then_0`
      (for (_array_element _array_index) _servers_1
        (`/Engine/EditorBlueprintResources/StandardMacros.IsValid` _array_element
          (:`Is Valid`
            (`self.K2_DestroyActor` _array_element)
            (`KismetArrayLibrary.Array_Remove` _servers_1 _array_index)))))
    (:`then_1`
      (for (_array_element_2 _array_index_2) _servers_2
        (`/Engine/EditorBlueprintResources/StandardMacros.IsValid` _array_element_2
          (:`Is Valid`
            (`self.K2_DestroyActor` _array_element_2)
            (`KismetArrayLibrary.Array_Remove` _servers_2 _array_index_2)))))))

(fn `UserConstructionScript`)