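; BP_Server2 is a server prop for the server room whose status lights flicker at random.
; On BeginPlay it creates dynamic material instances for three colored status lights and a green power button, storing the status lights in an array.
; A looping timer, with its interval randomized once at start, calls UpdateLights to give each array material a random emission strength.
; The power button material is kept separate, so it does not flicker.
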(event `self.ReceiveBeginPlay`
  (bind _matarray (`self.MatArray`))
  (`KismetSystemLibrary.K2_SetTimer` null "UpdateLights" (`KismetMathLibrary.RandomFloatInRange` 1.0 5.0) true)
  ; Create Mat Instances
  ;; Light 2
  (bind _returnvalue (`PrimitiveComponent.CreateDynamicMaterialInstance` (`self.SrvLight2`) 0 "/Game/GPP/Blueprints/ServerRoom/ServerRack/MI_ServerLightMaterial.MI_ServerLightMaterial" "None"))
  (`MaterialInstanceDynamic.SetVectorParameterValue` _returnvalue "Base Color" (struct :`G` 1.0 :`B` 0.020532 :`A` 1.0))
  (`KismetArrayLibrary.Array_Add` _matarray _returnvalue)
  ;; Light 1
  (bind _returnvalue_2 (`PrimitiveComponent.CreateDynamicMaterialInstance` (`self.SrvLight1`) 0 "/Game/GPP/Blueprints/ServerRoom/ServerRack/MI_ServerLightMaterial.MI_ServerLightMaterial" "None"))
  (`MaterialInstanceDynamic.SetVectorParameterValue` _returnvalue_2 "Base Color" (struct :`R` 1.0 :`B` 0.009094 :`A` 1.0))
  (`KismetArrayLibrary.Array_Add` _matarray _returnvalue_2)
  ;; Light 0
  (bind _returnvalue_3 (`PrimitiveComponent.CreateDynamicMaterialInstance` (`self.SrvLight`) 0 "/Game/GPP/Blueprints/ServerRoom/ServerRack/MI_ServerLightMaterial.MI_ServerLightMaterial" "None"))
  (`MaterialInstanceDynamic.SetVectorParameterValue` _returnvalue_3 "Base Color" (struct :`R` 1.0 :`G` 0.43476 :`A` 1.0))
  (`KismetArrayLibrary.Array_Add` _matarray _returnvalue_3)
  ;; Pwr Light
  (bind _returnvalue_4 (`PrimitiveComponent.CreateDynamicMaterialInstance` (`self.PwrBtn`) 0 "/Game/GPP/Blueprints/ServerRoom/ServerRack/MI_ServerLightMaterial.MI_ServerLightMaterial" "None"))
  (bind _output_get (set `self.PowerMat` _returnvalue_4))
  (`MaterialInstanceDynamic.SetVectorParameterValue` _output_get "Base Color" (struct :`R` 0.021185 :`G` 0.3125 :`B` 0.015294 :`A` 1.0)))

(event `UpdateLights`
  (for _array_element (`self.MatArray`)
    (`MaterialInstanceDynamic.SetScalarParameterValue` _array_element "EmissionStrength" (`KismetMathLibrary.RandomFloatInRange` 0.0 1.2))))

(fn `UserConstructionScript`)