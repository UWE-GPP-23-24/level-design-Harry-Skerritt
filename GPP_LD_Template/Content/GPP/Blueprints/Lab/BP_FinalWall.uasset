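; BP_FinalWall is a wall actor that lowers itself once its DropWall event is triggered.
; DropWall sets an IsDropping flag, and Tick then moves the actor along local Z by DropSpeed scaled by delta time, without sweep.
; The movement stops when the actor's world Z falls below StopZ.
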(event `DropWall`
  ; Trigger
  (set `self.IsDropping` true))

(event `self.ReceiveBeginPlay`
  ; Init
  (set `self.IsDropping` false))

(event `self.ReceiveTick`
  (params (DeltaSeconds :type "Float (single-precision)"))
  ; Logic
  (if (`self.IsDropping`)
    (`self.K2_AddActorLocalOffset` (`KismetMathLibrary.MakeVector` 0.0 0.0 (* DeltaSeconds (`self.DropSpeed`))))
    ; Stop When Finished
    (if (not (>= (.z (`self.K2_GetActorLocation` self)) (`self.StopZ`)))
      (set `self.IsDropping` false))))

(fn `UserConstructionScript`)