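; BP_OfficeRoomStartTrigger is a one-shot box trigger that starts an office room sequence, dropping the floor and activating moving platforms.
; The first overlap by any actor sets a Triggered flag, then destroys DropFloor after StartDelay.
; Without waiting for that delay, it casts each Platforms entry to BP_MovingPlatform_Simple_Large and calls StartPlatformMoving on it.
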(event `self.Box.OnComponentBeginOverlap`
  (params (OverlappedComponent :type "PrimitiveComponent Object Reference") (OtherActor :type "Actor Object Reference") (OtherComp :type "PrimitiveComponent Object Reference") (OtherBodyIndex :type Integer) (bFromSweep :type Boolean) (SweepResult :type "HitResult Structure (by ref)"))
  (bind _platforms (`self.Platforms`))
  (if (not (`self.Triggered`))
    (set `self.Triggered` true)
    (`|ExecutionSequence`
      (:`then_0`
        (`KismetSystemLibrary.Delay` (`self.StartDelay`))
        (`self.K2_DestroyActor` (`self.DropFloor`)))
      (:`then_1`
        ; Activate Platforms
        (if (`KismetArrayLibrary.Array_IsNotEmpty` _platforms)
          (for _array_element _platforms
            (bind _asbp_moving_platform_simple_large (cast `/Game/GPP/Blueprints/Platforms/BP_MovingPlatform_Simple_Large` _array_element))
            (`/Game/GPP/Blueprints/Platforms/BP_MovingPlatform_Simple_Large.StartPlatformMoving` _asbp_moving_platform_simple_large)))))))

(fn `UserConstructionScript`)