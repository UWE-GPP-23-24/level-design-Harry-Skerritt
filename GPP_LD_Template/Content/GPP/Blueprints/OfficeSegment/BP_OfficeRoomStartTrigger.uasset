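; BP_OfficeRoomStartTrigger is a one-shot trigger volume for the office segment that starts the collapse of a drop floor.
; The first box overlap sets a Triggered flag and calls ShakeAndBreak on DropFloor, with no filter on the overlapping actor.
; IsTriggered exposes that flag.
; Disconnected leftover nodes for adding score and starting moving platforms never run.
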(event `self.Box.OnComponentBeginOverlap`
  (params (OverlappedComponent :type "PrimitiveComponent Object Reference") (OtherActor :type "Actor Object Reference") (OtherComp :type "PrimitiveComponent Object Reference") (OtherBodyIndex :type Integer) (bFromSweep :type Boolean) (SweepResult :type "HitResult Structure (by ref)"))
  ; Conditional Triggering
  (if (not (`self.Triggered`))
    (set `self.Triggered` true)
    ; Trigger Platform
    (`/Game/GPP/Blueprints/OfficeSegment/OfficeFloor/BP_OfficeFloor.ShakeAndBreak` (`self.DropFloor`))))

(fn `IsTriggered`
  (returns (ColliderTriggered :type Boolean))
  (return (`self.Triggered`)))

(fn `UserConstructionScript`)