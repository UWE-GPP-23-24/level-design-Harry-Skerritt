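; BP_OfficeFloor is an office floor actor that shakes and then breaks away when ShakeAndBreak is triggered.
; It plays a rumble sound, starts a camera shake, and runs the Rumble timeline to randomly jitter the actor around its BeginPlay position.
; After ShakeDuration, it stops the camera shake immediately, destroys itself and plays the break sound.
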(event `self.ReceiveBeginPlay`
  ; Init Pos
  (set `self.StartPosition` (`self.K2_GetActorLocation`)))

(event `ShakeAndBreak`
  ; Shake and Break
  (`|ExecutionSequence`
    (:`then_0`
      (`GameplayStatics.PlaySound2D` "/Game/GPP/Blueprints/OfficeSegment/OfficeFloor/MS_FloorRumble.MS_FloorRumble" 1.0 1.0 0.0 null null)
      ;; Break
      (`KismetSystemLibrary.Delay` (`self.ShakeDuration`))
      (`PlayerCameraManager.StopCameraShake` (`GameplayStatics.GetPlayerCameraManager` 0) (`self.Camera Shake`) true)
      (`|ExecutionSequence`
        (:`then_0`
          (`self.K2_DestroyActor`))
        (:`then_1`
          (`GameplayStatics.PlaySound2D` "/Game/GPP/Blueprints/OfficeSegment/OfficeFloor/MS_FloorBreak.MS_FloorBreak" 1.0 1.0 0.0 null null))))
    (:`then_1`
      (`|ExecutionSequence`
        (:`then_0`
          ;; Shake Logic
          (`Timeline|Rumble`
            (:`Update`
              (`self.K2_SetActorLocation` (+ (`self.StartPosition`) (* (`self.ShakeIntensity`) (`KismetMathLibrary.RandomFloatInRange` -1.0 1.0)))))))
        (:`then_1`
          ;; Add Camera Shake
          (bind _returnvalue (`PlayerCameraManager.StartCameraShake` :`self` (`GameplayStatics.GetPlayerCameraManager` 0) :`ShakeClass` "/Game/GPP/Blueprints/OfficeSegment/OfficeFloor/BP_OfficeCameraShake.BP_OfficeCameraShake_C"))
          (set `self.Camera Shake` _returnvalue))))))

(fn `UserConstructionScript`)