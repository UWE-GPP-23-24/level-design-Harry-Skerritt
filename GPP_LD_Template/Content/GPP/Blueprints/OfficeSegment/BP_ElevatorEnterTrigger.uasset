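; Trigger volume in the office segment's elevator that completes the current mission and fakes an elevator ride down.
; When something overlaps its box, it notifies the MissionManager, closes the elevator doors after a short pause, then steps the floor sign from 0 through G to -1 on a shared delay.
; It finishes by opening a separate set of exit doors.
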(event `self.Box.OnComponentBeginOverlap`
  (params (OverlappedComponent :type "PrimitiveComponent Object Reference") (OtherActor :type "Actor Object Reference") (OtherComp :type "PrimitiveComponent Object Reference") (OtherBodyIndex :type Integer) (bFromSweep :type Boolean) (SweepResult :type "HitResult Structure (by ref)"))
  (bind _sign (`self.Sign`))
  (bind _signdelay (`self.SignDelay`))
  (`/Game/GPP/Blueprints/Missions/BP_MissionManager.CompleteMission` (`self.MissionManager`))
  (`KismetSystemLibrary.Delay` 1.0)
  (`/Game/GPP/Blueprints/ElevatorSection/BP_ElevatorDoors.Close Door` (`self.ElevatorDoors`))
  (`KismetSystemLibrary.Delay` (* _signdelay 2.0))
  (`/Game/GPP/Blueprints/ElevatorSection/BP_ElevatorSign.SetFloorNo` _sign "0")
  (`KismetSystemLibrary.Delay` _signdelay)
  (`/Game/GPP/Blueprints/ElevatorSection/BP_ElevatorSign.SetFloorNo` _sign "G")
  (`KismetSystemLibrary.Delay` _signdelay)
  (`/Game/GPP/Blueprints/ElevatorSection/BP_ElevatorSign.SetFloorNo` _sign "-1")
  (`KismetSystemLibrary.Delay` _signdelay)
  (`/Game/GPP/Blueprints/ElevatorSection/BP_ElevatorDoors.Open Door` (`self.ElevatorDoorsOut`)))

(fn `UserConstructionScript`)