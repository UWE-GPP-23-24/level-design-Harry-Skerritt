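; Office-segment trigger volume that starts a set of moving desk platforms when something overlaps its box.
; The first overlap latches a one-shot flag, then starts the platforms only if the referenced StartTrigger has already been triggered.
; Because the flag is set before that check, an early overlap uses up the trigger without moving anything.
; Each entry in the Platforms array is cast to BP_MovingPlatform_Desk to call StartPlatformMoving.
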(event `self.Box.OnComponentBeginOverlap`
  (params (OverlappedComponent :type "PrimitiveComponent Object Reference") (OtherActor :type "Actor Object Reference") (OtherComp :type "PrimitiveComponent Object Reference") (OtherBodyIndex :type Integer) (bFromSweep :type Boolean) (SweepResult :type "HitResult Structure (by ref)"))
  (bind _platforms (`self.Platforms`))
  ; Conditional Trigger
  (if (not (`self.Triggered`))
    (set `self.Triggered` true)
    ; Check other trigger triggered
    (bind _collidertriggered (`/Game/GPP/Blueprints/OfficeSegment/BP_OfficeRoomStartTrigger.IsTriggered` (`self.StartTrigger`)))
    (if _collidertriggered
      ; Activate Platforms
      (if (`KismetArrayLibrary.Array_IsNotEmpty` _platforms)
        (for _array_element _platforms
          (bind _asbp_moving_platform_desk (cast `/Game/GPP/Blueprints/Platforms/BP_MovingPlatform_Desk` _array_element))
          (`/Game/GPP/Blueprints/Platforms/BP_MovingPlatform_Desk.StartPlatformMoving` _asbp_moving_platform_desk))))))

(fn `UserConstructionScript`)